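; AI controller for a monster that runs the BT_Clot behavior tree when it possesses its pawn.
; AI perception updates write whether the stimulus was sensed to the IsPlayerVisible blackboard key, without checking which actor triggered it.
; While the IsRotate flag is on, Tick smoothly turns the pawn's yaw toward the first player's pawn using RInterpTo.
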(event `self.ReceivePossess`
  (params (PossessedPawn :type "Pawn Object Reference"))
  (`self.RunBehaviorTree` "/Game/AI/BT_Clot.BT_Clot"))

(event `self.ReceiveTick`
  (params (DeltaSeconds :type "Float (single-precision)"))
  (bind _returnvalue (`GameplayStatics.GetPlayerPawn` 0))
  (if (`self.IsRotate`)
    (`/Engine/EditorBlueprintResources/StandardMacros.IsValid` _returnvalue
      (:`Is Valid`
        (bind (_returnvalue_roll _returnvalue_pitch _returnvalue_yaw) (`KismetMathLibrary.BreakRotator` (`KismetMathLibrary.RInterpTo` (`self.K2_GetActorRotation` (stale `self.ReceivePossess` PossessedPawn)) (`KismetMathLibrary.FindLookAtRotation` (`self.K2_GetActorLocation` (stale `self.ReceivePossess` PossessedPawn)) (`self.K2_GetActorLocation` _returnvalue)) DeltaSeconds 20.0)))
        (`self.K2_SetActorRotation` (stale `self.ReceivePossess` PossessedPawn) (`KismetMathLibrary.MakeRotator` 0.0 0.0 _returnvalue_yaw) false)))))

(event `self.AIPerception.OnTargetPerceptionUpdated`
  (params (Actor :type "Actor Object Reference") (Stimulus :type "AIStimulus Structure"))
  ; Skill(TODO)
  (`BlackboardComponent.SetValueAsBool` (`AIBlueprintHelperLibrary.GetBlackboard` null) "IsPlayerVisible" (`.bSuccessfullySensed` (break `AIStimulus` Stimulus))))

(fn `UserConstructionScript`)