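; Game mode for a Killing Floor-like wave game that starts waves and reports their progress to the HUD.
; On BeginPlay it caches the first player's BP_PlayerCharacterController, waits one tick, then calls StartWave, whose logic lives outside this graph.
; Wave and remaining-monster update events pass the game mode to the controller's WBCrosshair widget, if valid, to refresh its display.
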(event `self.ReceiveBeginPlay`
  (bind _asbp_player_character_controller (cast `/Game/BluePrint/BP_PlayerCharacterController` (`Pawn.GetController` (`GameplayStatics.GetPlayerPawn` 0))))
  (set `self.PlayerCharacterController` _asbp_player_character_controller)
  (`KismetSystemLibrary.DelayUntilNextTick`)
  (`self.StartWave`))

(event `self.OnUpdateRemainMonsterCount`
  (bind _wb_crosshair (`/Game/BluePrint/BP_PlayerCharacterController.WB_Crosshair` (`self.PlayerCharacterController`)))
  (`/Engine/EditorBlueprintResources/StandardMacros.IsValid` _wb_crosshair
    (:`Is Valid`
      (`/Game/UI/WB_Crosshair.UpdateRemainMonster` _wb_crosshair self))))

(event `self.OnUpdateWave`
  (bind _wb_crosshair (`/Game/BluePrint/BP_PlayerCharacterController.WB_Crosshair` (`self.PlayerCharacterController`)))
  (`/Engine/EditorBlueprintResources/StandardMacros.IsValid` _wb_crosshair
    (:`Is Valid`
      (`/Game/UI/WB_Crosshair.UpdateWave` _wb_crosshair self))))

(fn `UserConstructionScript`)