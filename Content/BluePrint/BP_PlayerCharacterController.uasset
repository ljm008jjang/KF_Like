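; Player controller for the first-person character that adds the crosshair widget to the viewport on BeginPlay and relays weapon-swap input.
; When IA_SwapWeapon starts, it waits one tick, then passes the truncated input value to the controlled BP_FirstPersonCharacter as the swap request.
; IA_WeaponAim is empty; logic toggling the current weapon between Normal and Iron aim exists but is disconnected and never runs.
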(event `self.ReceiveBeginPlay`
  (bind _returnvalue (`|CreateWidget` "/Game/UI/WB_Crosshair.WB_Crosshair_C"))
  (`UserWidget.AddToViewport` _returnvalue 0))

(event `EnhancedInput|/Game/FirstPerson/Input/Actions/IA_SwapWeapon`
  (params (ActionValue :type "Float (double-precision)") (ElapsedSeconds :type "Float (double-precision)") (TriggeredSeconds :type "Float (double-precision)") (InputAction :type "InputAction Object Reference" :default "/Game/FirstPerson/Input/Actions/IA_SwapWeapon.IA_SwapWeapon"))
  (:`Triggered`
    (if true
      _))
  (:`Started`
    (`KismetSystemLibrary.DelayUntilNextTick`)
    (bind _asbp_first_person_character (cast `/Game/BluePrint/Character/BP_FirstPersonCharacter` (`self.K2_GetPawn`)))
    (`KillingFloorLikeCharacter.OnTriggerSwapWeapon` _asbp_first_person_character (`KismetMathLibrary.FTrunc` ActionValue))))

(event `EnhancedInput|/Game/FirstPerson/Input/Actions/IA_WeaponAim`
  (params (ActionValue :type Boolean) (ElapsedSeconds :type "Float (double-precision)") (TriggeredSeconds :type "Float (double-precision)") (InputAction :type "InputAction Object Reference" :default "/Game/FirstPerson/Input/Actions/IA_WeaponAim.IA_WeaponAim")))

(fn `UserConstructionScript`)