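; BP_Stalker is a child character Blueprint for a stalker that starts out transparent and reveals itself when it attacks or takes damage.
; BeginPlay, AnyDamage and OnAttackEvent each run the parent logic, then call ChangeMaterial.
; ChangeMaterial swaps the first two mesh material slots between a shared transparent material and the default and hair materials.
; Nothing in this Blueprint restores transparency after the reveal.
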(event `self.ReceiveBeginPlay`
  (`parent.ReceiveBeginPlay`)
  (`self.ChangeMaterial` true))

(event `self.ReceiveAnyDamage`
  (params (Damage :type "Float (single-precision)") (DamageType :type "DamageType Object Reference") (InstigatedBy :type "Controller Object Reference") (DamageCauser :type "Actor Object Reference"))
  (`parent.ReceiveAnyDamage` Damage DamageType InstigatedBy DamageCauser)
  (`self.ChangeMaterial` false))

(event `self.OnAttackEvent`
  (`parent.OnAttackEvent`)
  (`self.ChangeMaterial` false))

(fn `ChangeMaterial`
  (params (IsTransparent :type Boolean))
  (bind _mesh (`self.Mesh`))
  (bind _transparentmaterial (`self.TransparentMaterial`))
  (bind _mesh_2 (`self.Mesh`))
  (if IsTransparent
    (`PrimitiveComponent.SetMaterial` _mesh_2 0 _transparentmaterial)
    (`PrimitiveComponent.SetMaterial` _mesh_2 1 _transparentmaterial)
    (return)
    (else
      (`PrimitiveComponent.SetMaterial` _mesh 0 (`self.DefaultMaterial`))
      (`PrimitiveComponent.SetMaterial` _mesh 1 (`self.HairMaterial`)))))

(fn `UserConstructionScript`
  (`parent.UserConstructionScript`))