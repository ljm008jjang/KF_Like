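; BP_Fleshpound is the Blueprint for the Fleshpound enemy character, which switches into a rage state when badly hurt.
; On damage, unless already in the Run state, it waits a tick and checks whether health is at or below half.
; If so, it plays a rage montage, changes to Run and holds the IsChangingRage blackboard flag until the montage completes or is interrupted.
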(event `self.ReceiveAnyDamage`
  (params (Damage :type "Float (single-precision)") (DamageType :type "DamageType Object Reference") (InstigatedBy :type "Controller Object Reference") (DamageCauser :type "Actor Object Reference"))
  (bind _returnvalue (`AIBlueprintHelperLibrary.GetBlackboard` null))
  (`parent.ReceiveAnyDamage` Damage DamageType InstigatedBy DamageCauser)
  (if (`|EnumInequality` (`self.CurrentUnitState`) (enumliteral `EUnitState` "Run"))
    (`KismetSystemLibrary.DelayUntilNextTick`)
    (bind _returnvalue_2 (`self.GetHpRatio`))
    (if (<= _returnvalue_2 0.5)
      (`BlackboardComponent.SetValueAsBool` _returnvalue "IsChangingRage" true)
      (`|PlayMontage` (`self.Mesh`) "/Game/KF/Character/KF_Freaks_Trip/Fleshpound/PoundRage_Montage.PoundRage_Montage"
        (:`then`
          (`self.ChangeUnitState` "Run"))
        (:`OnCompleted`
          (`BlackboardComponent.SetValueAsBool` _returnvalue "IsChangingRage" false :!label _label))
        (:`OnInterrupted`
          (goto _label))))))

(fn `UserConstructionScript`
  (`parent.UserConstructionScript`))