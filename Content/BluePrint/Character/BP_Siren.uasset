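; BP_Siren is a character Blueprint whose skill deals radial damage around its own location.
; On DoSkill, a sphere overlap gathers nearby Monster pawns and passes them as the ignore list to ApplyRadialDamage over the same radius, so those monsters are spared.
; The Siren and its controller are credited as causer and instigator, and WorldStatic geometry can block the damage.
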(event `self.DoSkill`
  (bind _returnvalue (`self.K2_GetActorLocation`))
  (bind _outactors (`KismetSystemLibrary.SphereOverlapActors` _returnvalue 500.0 (`|MakeArray` "ObjectTypeQuery3" :!type "EObjectTypeQuery Enum") "/Script/KillingFloorLike.Monster"))
  (`GameplayStatics.ApplyRadialDamage` 30.0 _returnvalue 500.0 null _outactors self (`self.GetController`) false "ECC_WorldStatic"))

(fn `UserConstructionScript`
  (`parent.UserConstructionScript`))