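; Behavior Tree task that makes a monster play an attack montage while the blackboard's Player is alive.
; It picks a montage by random index from the monster's set for the configured AnimType.
; The AI controller's IsRotate flag is raised for playback and lowered afterwards, with completion reporting success and interruption failure.
; If the player is dead, it clears the Player key and fails.
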(event `self.ReceiveExecute`
  (params (OwnerActor :type "Actor Object Reference"))
  (bind _returnvalue (`AIBlueprintHelperLibrary.GetAIController` OwnerActor))
  (bind _blackboardkeyselector (make `BlackboardKeySelector` :`SelectedKeyName` "Player"))
  (bind _animtype (`self.AnimType`))
  (bind _askilling_floor_like_character (cast `KillingFloorLikeCharacter` (`BTFunctionLibrary.GetBlackboardValueAsObject` _blackboardkeyselector)))
  (bind _returnvalue_2 (`BaseCharacter.GetIsAlive` _askilling_floor_like_character))
  (if _returnvalue_2
    (bind _asbp_monster_aicontroller (cast `/Game/BluePrint/BP_MonsterAIController` _returnvalue))
    (bind _asmonster (cast `Monster` (`Controller.K2_GetPawn` _returnvalue)))
    (bind _returnvalue_3 (`Monster.GetAnimationMaxIndex` _asmonster _animtype))
    (bind _returnvalue_4 (`Monster.GetAnimationMontage` _asmonster _animtype (`KismetMathLibrary.RandomInteger` _returnvalue_3)))
    (set `/Game/BluePrint/BP_MonsterAIController.IsRotate` true _asbp_monster_aicontroller)
    (`|PlayMontage` (`Character.Mesh` _asmonster) _returnvalue_4
      (:`OnCompleted`
        (`self.FinishExecute` true))
      (:`OnInterrupted`
        (`self.FinishExecute` false)))
    (`/Engine/EditorBlueprintResources/StandardMacros.IsValid` _asbp_monster_aicontroller
      (:`Is Valid`
        (set `/Game/BluePrint/BP_MonsterAIController.IsRotate` false _asbp_monster_aicontroller)))
    (else
      (`BTFunctionLibrary.ClearBlackboardValue` _blackboardkeyselector)
      (`self.FinishExecute` false))))