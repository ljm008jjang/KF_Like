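; Behavior Tree task that plays a Husk monster's skill animation.
; On execute it gets the AI controller and controlled Monster, fetches the first Skill montage, sets the controller's IsRotate flag and plays the montage on the mesh.
; Completion finishes the task as success and interruption as failure, both clearing IsRotate.
; A failed cast stops execution without finishing the task.
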(event `self.ReceiveExecute`
  (params (OwnerActor :type "Actor Object Reference"))
  (bind _returnvalue (`AIBlueprintHelperLibrary.GetAIController` OwnerActor))
  (bind _asbp_monster_aicontroller (cast `/Game/BluePrint/BP_MonsterAIController` _returnvalue))
  (bind _asmonster (cast `Monster` (`Controller.K2_GetPawn` _returnvalue)))
  (bind _returnvalue_2 (`Monster.GetAnimationMontage` _asmonster "Skill" 0))
  (set `/Game/BluePrint/BP_MonsterAIController.IsRotate` true _asbp_monster_aicontroller)
  (`|PlayMontage` (`Character.Mesh` _asmonster) _returnvalue_2
    (:`OnCompleted`
      (`self.FinishExecute` true))
    (:`OnInterrupted`
      (`self.FinishExecute` false)))
  (set `/Game/BluePrint/BP_MonsterAIController.IsRotate` false _asbp_monster_aicontroller))